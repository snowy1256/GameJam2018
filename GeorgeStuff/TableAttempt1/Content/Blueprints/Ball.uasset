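; Physics ball actor that pushes itself along the world Y axis and clings to the surface beneath it.
; Each tick, a frame-time-scaled velocity impulse drives it away from a hard-coded Y dividing line, in whichever direction matches its side.
; A short downward trace supplies the surface normal for a second impulse that pulls the ball into that surface.
; Its linear velocity is then clamped to a maximum speed.
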(event `self.ReceiveBeginPlay`)

(event `self.ReceiveTick`
  (params (DeltaSeconds :type "Float (single-precision)"))
  (bind _returnvalue (`self.K2_GetActorLocation`))
  (`PrimitiveComponent.AddImpulse` (`self.Ball`) (`KismetMathLibrary.MakeVector` 0.0 (* (- (* (`KismetMathLibrary.Conv_BoolToDouble` (> (.y (`self.K2_GetActorLocation`)) -650.0)) 2.0) 1.0) DeltaSeconds 1500.0) 0.0) "None" true)
  (bind _outhit (`KismetSystemLibrary.LineTraceSingle` _returnvalue (+ _returnvalue (0.0 0.0 -250.0)) "TraceTypeQuery1"))
  (`PrimitiveComponent.AddImpulse` (`self.Ball`) (* (* (`.ImpactNormal` (`GameplayStatics.BreakHitResult` _outhit)) -1.0) (* 1000.0 DeltaSeconds)) "None" true)
  (bind _returnvalue_2 (`PrimitiveComponent.GetPhysicsLinearVelocity` (`self.Ball`) "None"))
  (`PrimitiveComponent.SetPhysicsLinearVelocity` (`self.Ball`) (`KismetMathLibrary.ClampVectorSize` _returnvalue_2 0.0 4000.0) false "None"))

(fn `UserConstructionScript`)