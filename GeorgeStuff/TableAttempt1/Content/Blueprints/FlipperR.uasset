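; Right pinball-style flipper actor that swings up while Right Ctrl is held and drops back when released.
; BeginPlay enables player input, and the key events set an Activate flag read on Tick.
; Tick snaps yaw to fixed end stops, otherwise rotates by a frame-time-scaled step.
; NOR conditions converted to floats pick the direction without branching, with the return stroke slightly slower than the outward one.
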(event `self.ReceiveBeginPlay`
  ;[1 1 1] Enable Control Input
  (`self.EnableInput` (`GameplayStatics.GetPlayerController` 0)))

(event `Key|RightControl`
  (params (Key :type "Key Structure"))
  ;[1 1 1] Handle Keypress
  (:`Pressed`
    (set `self.Activate` true))
  (:`Released`
    (set `self.Activate` false)))

(event `self.ReceiveTick`
  (params (DeltaSeconds :type "Float (single-precision)"))
  (bind _activate (`self.Activate`))
  (bind _returnvalue (not _activate))
  (bind _roll (.roll (`self.K2_GetActorRotation`)))
  (bind _pitch (.pitch (`self.K2_GetActorRotation`)))
  (bind _yaw (.yaw (`self.K2_GetActorRotation`)))
  (bind _returnvalue_2 (>= _yaw -60.0))
  (bind _returnvalue_3 (<= _yaw -100.0))
  ;[1 1 1] Rotate in steps
  (if (and _returnvalue_2 _activate)
    (`self.K2_SetActorRotation` (`KismetMathLibrary.MakeRotator` _roll _pitch -60.0))
    (elif (and _returnvalue_3 _returnvalue)
      (`self.K2_SetActorRotation` (`KismetMathLibrary.MakeRotator` _roll _pitch -100.0))
      (else
        (`self.K2_AddActorLocalRotation` (`KismetMathLibrary.MakeRotator` 0.0 0.0 (* (+ (`KismetMathLibrary.Conv_BoolToDouble` (`KismetMathLibrary.BooleanNOR` _returnvalue _returnvalue_2)) (* (`KismetMathLibrary.Conv_BoolToDouble` (`KismetMathLibrary.BooleanNOR` _activate _returnvalue_3)) -0.8)) 2000.0 DeltaSeconds)))))))

(fn `UserConstructionScript`)