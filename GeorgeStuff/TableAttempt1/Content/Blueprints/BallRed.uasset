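; BallRed is a red ball actor that registers itself with the level's shared state when it spawns.
; On BeginPlay it runs the parent logic, then takes the first LevelDatabase actor found in the world.
; It sets RedInPlay on that database and decrements its RedBalls count by one.
; All other behavior comes from the parent class, as the overlap and tick events here are disabled.
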(event `self.ReceiveBeginPlay`
  (`parent.ReceiveBeginPlay`)
  (bind _outactors (`GameplayStatics.GetAllActorsOfClass` "/Game/Blueprints/LevelDatabase.LevelDatabase_C"))
  (bind _output (`|GetArrayItem` _outactors))
  (set `/Game/Blueprints/LevelDatabase.redInPlay` true _output)
  (set `/Game/Blueprints/LevelDatabase.redBalls` (- (`/Game/Blueprints/LevelDatabase.redBalls` _output) 1) _output))

(fn `UserConstructionScript`
  (`parent.UserConstructionScript`))