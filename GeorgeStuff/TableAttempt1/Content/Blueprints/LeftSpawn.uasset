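; LeftSpawn is an actor that launches blue balls into the level on player input.
; It enables input for the first player controller and listens for the LeftBallLaunch action.
; On press, it reads the first LevelDatabase actor and spawns BallBlue at a hardcoded location, only if blue balls remain and none is in play.
; It does not update those counters itself.
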(event `self.ReceiveBeginPlay`
  (`self.EnableInput` (`GameplayStatics.GetPlayerController` 0)))

(event `InputAction|LeftBallLaunch`
  (params (Key :type "Key Structure"))
  (:`Pressed`
    (bind _outactors (`GameplayStatics.GetAllActorsOfClass` "/Game/Blueprints/LevelDatabase.LevelDatabase_C"))
    (bind _output (`|GetArrayItem` _outactors))
    (if (and (> (`/Game/Blueprints/LevelDatabase.blueBalls` _output) 0) (not (`/Game/Blueprints/LevelDatabase.blueInPlay` _output)))
      (`|SpawnActorFromClass` "/Game/Blueprints/BallBlue.BallBlue_C" (`KismetMathLibrary.MakeTransform` (1600.0 -78.699997 518.0) (struct)) "Undefined" "OverrideRootScale" null null))))

(fn `UserConstructionScript`)