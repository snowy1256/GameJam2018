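; Test actor that spins a physics-simulated Flipper component by applying a torque impulse on a key press.
; BeginPlay enables player input, and pressing H sets an Activate flag that Tick consumes once, adding a very large yaw-axis torque in degrees to Bone001.
; Releasing H clears the flag, so each press yields at most one frame of torque.
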(event `self.ReceiveBeginPlay`
  ;[1 1 1] Enable Control Input
  (`self.EnableInput` (`GameplayStatics.GetPlayerController` 0)))

(event `Key|H`
  (params (Key :type "Key Structure"))
  ;[1 1 1] Handle Keypress
  (:`Pressed`
    (set `self.Activate` true))
  (:`Released`
    (set `self.Activate` false)))

(event `self.ReceiveTick`
  (params (DeltaSeconds :type "Float (single-precision)"))
  (if (`self.Activate`)
    (set `self.Activate` false)
    (`PrimitiveComponent.AddTorqueInDegrees` (`self.Flipper`) (0.0 0.0 50000000188416.0) "Bone001" false)))

(fn `UserConstructionScript`)