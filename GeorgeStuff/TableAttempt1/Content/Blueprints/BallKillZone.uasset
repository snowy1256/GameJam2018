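; BallKillZone is an overlap trigger that removes Ball actors from play and awards points.
; On overlap it casts to Ball, clears that colour's in-play flag on the first LevelDatabase found in the level, then destroys the ball.
; A fixed world Y threshold decides the side: a ball ending on the opposing side adds a fixed bonus to its colour's score.
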(event `self.ReceiveActorBeginOverlap`
  (params (OtherActor :type "Actor Object Reference"))
  (bind _asball (cast `/Game/Blueprints/Ball` OtherActor))
  (bind _outactors (`GameplayStatics.GetAllActorsOfClass` "/Game/Blueprints/LevelDatabase.LevelDatabase_C"))
  ;[1 1 1] Is blue?
  (if (`/Game/Blueprints/Ball.isBlue` _asball)
    (bind _output (`|GetArrayItem` _outactors))
    (set `/Game/Blueprints/LevelDatabase.blueInPlay` false _output)
    (bind _returnvalue (> (.y (`self.K2_GetActorLocation` _asball)) -650.0))
    (if _returnvalue
      (set `/Game/Blueprints/LevelDatabase.blueScore` (+ (`/Game/Blueprints/LevelDatabase.blueScore` _output) 10000) _output))
    (else
      (set `/Game/Blueprints/LevelDatabase.redInPlay` false _output)
      (if (not _returnvalue)
        (set `/Game/Blueprints/LevelDatabase.redScore` (+ 10000 (`/Game/Blueprints/LevelDatabase.redScore` _output)) _output))))
  (`self.K2_DestroyActor` _asball))

(fn `UserConstructionScript`)